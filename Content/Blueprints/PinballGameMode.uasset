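; Pinball game mode that runs a match: ball supply, multiplied score, game over and reset, with looping-named music started at BeginPlay.
; Balls spawn at the plunger, and each one's destruction triggers a respawn or ends the game when none remain.
; Game over opens a high-score entry widget if the saved list is short or the score beats its lowest, using a cached, load-or-create save object.
; Reset restores class defaults, spawns a ball and recreates the HUD.
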(event `self.ReceiveBeginPlay`
  (`self.SpawnBall`)
  (`GameplayStatics.PlaySound2D` "/Game/Assets/Sounds/victoryMusic_loop_01_01.victoryMusic_loop_01_01" 0.03))

(event `SpawnBall`
  (bind _outactors (`GameplayStatics.GetAllActorsOfClass` "/Game/Blueprints/BP_Plunger.BP_Plunger_C"))
  (bind _returnvalue (`|SpawnActorFromClass` "/Game/Blueprints/BP_Ball.BP_Ball_C" (`KismetMathLibrary.MakeTransform` (`/Game/Blueprints/BP_Plunger.GetBallSpawnLocation` (`|GetArrayItem` _outactors))) "Undefined" "OverrideRootScale" null null))
  (add `self.OnDestroyed` _returnvalue (delegate `OnBallDestroyed`)))

(event `OnBallDestroyed`
  (params (DestroyedActor :type "Actor Object Reference"))
  (if (>= (`self.BallsRemaining`) 0)
    (`self.SpawnBall`)
    (`/Engine/EditorBlueprintResources/StandardMacros.DecrementInt` (`self.BallsRemaining`))
    (else
      (`self.EndGame`))))

(event `EndGame`
  (bind _currentsaveobject (`self.GetSaveGameData`))
  (if (<= (`KismetArrayLibrary.Array_Length` (`/Game/Blueprints/HighScoreSave.SaveStruct` _currentsaveobject)) 3)
    (`self.CreateHighScoresList` :!label _label)
    (else
      (bind _lowestscorestruct (`/Game/Blueprints/HighScoreSave.DetermineLowestScoreValue` _currentsaveobject))
      (if (< (`.Score_6_B4CF239C220C090D002303B84E76052F` (break `/Game/Blueprints/HighScoreStruct` _lowestscorestruct)) (`self.Score`))
        (goto _label)))))

(event `CreateHighScoresList`
  (bind _aspinball_player_controller (cast `/Game/Blueprints/PinballPlayerController` (`GameplayStatics.GetPlayerController` 0) :!pure true))
  (bind _returnvalue (`|CreateWidget` "/Game/Blueprints/HighScoreEntry.HighScoreEntry_C" _aspinball_player_controller))
  (`UserWidget.AddToViewport` _returnvalue 0)
  (set `PlayerController.bShowMouseCursor` true _aspinball_player_controller)
  (`self.OnGameReset`))

(event `ResetGame`
  (bind (_score _multiplier _ballsremaining _highscoresavename _ongamereset _tiltcount) (defaults `/Game/Blueprints/PinballGameMode` "PinballGameMode_C"))
  (bind _aspinball_player_controller (cast `/Game/Blueprints/PinballPlayerController` (`GameplayStatics.GetPlayerController` 0) :!pure true))
  (set `self.Score` _score)
  (set `self.Multiplier` _multiplier)
  (set `self.BallsRemaining` _ballsremaining)
  (set `self.TiltCount` _tiltcount)
  (`self.SpawnBall`)
  (`/Game/Blueprints/PinballPlayerController.CreatePlayerHUD` _aspinball_player_controller)
  (set `PlayerController.bShowMouseCursor` false _aspinball_player_controller)
  (`self.OnGameReset`))

(fn `AddScore`
  (params (PointsToAdd :type "Float (double-precision)"))
  (returns (NewScore :type "Float (double-precision)"))
  (bind _output_get (set `self.Score` (+ (* PointsToAdd (`self.Multiplier`)) (`self.Score`))))
  (return _output_get))

(fn `GetSaveGameData`
  (returns (CurrentSaveObject :type "/Game/Blueprints/HighScoreSave Object Reference"))
  (bind _currentsaveobject (`self.CurrentSaveObject`)
    (:`then`
      (return _currentsaveobject))
    (:`else`
      (`GameplayStatics.DoesSaveGameExist` (`self.HighScoreSaveName`))
      (if true
        (bind _returnvalue (`GameplayStatics.LoadGameFromSlot` (`self.HighScoreSaveName`)))
        (bind _ashigh_score_save (cast `/Game/Blueprints/HighScoreSave` _returnvalue)
          (:`then`
            (`/Game/Blueprints/HighScoreSave.SortSaveData` _ashigh_score_save)
            (bind _output_get (set `self.CurrentSaveObject` _ashigh_score_save))
            (return _output_get))
          (:`CastFailed`
            (return null)))
        (else
          (bind _returnvalue_2 (`GameplayStatics.CreateSaveGameObject` "/Game/Blueprints/HighScoreSave.HighScoreSave_C"))
          (bind _output_get_2 (set `self.CurrentSaveObject` _returnvalue_2))
          (bind _returnvalue_3 (`GameplayStatics.SaveGameToSlot` _output_get_2 (`self.HighScoreSaveName`)))
          (if _returnvalue_3
            (return _output_get_2)
            (else
              (return null))))))))

(fn `UserConstructionScript`)