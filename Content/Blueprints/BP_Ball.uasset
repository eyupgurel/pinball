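; Pinball ball actor that drives itself with physics impulses and self-destructs when it stops getting anywhere.
; Each tick applies a default push plus a stickiness impulse against the traced surface normal below, spawns contact sparks, and scales rolling-sound volume and pitch by speed.
; A looping Locate timer sums displacement over a countdown, destroying the ball with sparks and sound if the total is under ExplosionThreshold.
; Destruction also triggers Explode sparks.
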(event `self.ReceiveBeginPlay`
  (`GameplayStatics.SpawnSoundAttached` "/Game/Assets/Sounds/Pinball_BallLoose_Cue.Pinball_BallLoose_Cue" (`self.Ball`))
  (`KismetSystemLibrary.K2_SetTimer` null "Locate" 1.0 true))

(event `self.ReceiveTick`
  (params (DeltaSeconds :type "Float (single-precision)"))
  (bind _returnvalue (`self.K2_GetActorLocation`))
  (bind _returnvalue_2 (/ (`KismetMathLibrary.VSize` (`self.GetVelocity`)) 1000.0))
  (`|ExecutionSequence`
    (:`then_0`
      (`PrimitiveComponent.AddImpulse` (`self.Ball`) (* (`self.DefaultSpeed`) DeltaSeconds) "None" true)
      (bind _outhit (`KismetSystemLibrary.LineTraceSingle` _returnvalue (- _returnvalue (0.0 0.0 500.0)) "TraceTypeQuery1"))
      (bind (_bblockinghit _binitialoverlap _time _distance _location _impactpoint _normal _impactnormal) (`GameplayStatics.BreakHitResult` _outhit))
      (`GameplayStatics.SpawnEmitterAtLocation` "/Game/Assets/ParticleSystems/PS_BallContactSparks.PS_BallContactSparks" _impactpoint)
      (`PrimitiveComponent.AddImpulse` (`self.Ball`) (* (* _impactnormal -1.0) (* (`self.TableStickyness`) DeltaSeconds)) "None" true))
    (:`then_1`
      (`AudioComponent.SetVolumeMultiplier` (`self.BallRollingSound`) (`KismetMathLibrary.FClamp` _returnvalue_2))
      (`AudioComponent.SetPitchMultiplier` (`self.BallRollingSound`) (`KismetMathLibrary.FClamp` _returnvalue_2 0.97 1.2)))))

(event `self.ReceiveDestroyed`
  (`self.Explode`))

(fn `Explode`
  (`GameplayStatics.SpawnEmitterAtLocation` "/Game/Assets/ParticleSystems/PS_BallExplosionSparks.PS_BallExplosionSparks" (`SceneComponent.K2_GetComponentLocation` (`self.Ball`))))

(fn `Locate`
  (bind (_defaultspeed _tablestickyness _location _cumulativedisplacement _counter _explosionthreshold) (defaults `/Game/Blueprints/BP_Ball` "BP_Ball_C"))
  (bind _cumulativedisplacement_2 (`self.CumulativeDisplacement`))
  (bind _returnvalue (`SceneComponent.K2_GetComponentLocation` (`self.Ball`)))
  (set `self.CumulativeDisplacement` (+ (`self.CumulativeDisplacement`) (`KismetMathLibrary.VSize` (- (`self.Location`) _returnvalue))))
  (set `self.Location` _returnvalue)
  (bind _result (`/Engine/EditorBlueprintResources/StandardMacros.DecrementInt` (`self.Counter`))
    (:`  `
      (if (== _result 0)
        (set `self.Counter` _counter)
        (if (< _cumulativedisplacement_2 _explosionthreshold)
          (`self.Explode`)
          (`GameplayStatics.PlaySoundAtLocation` "/Game/Assets/Sounds/Arcade_Enemy_Death_03_m1_Cue.Arcade_Enemy_Death_03_m1_Cue" (`self.K2_GetActorLocation`))
          (`self.K2_DestroyActor`)
          (else
            (`KismetSystemLibrary.PrintString` (`KismetStringLibrary.Conv_DoubleToString` _cumulativedisplacement_2))
            (set `self.CumulativeDisplacement` 0.0)))))))

(fn `UserConstructionScript`)